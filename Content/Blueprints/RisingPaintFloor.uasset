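; Rising paint floor hazard that kills the player on touch.
; It registers itself with PaintMode on BeginPlay and exposes BeginRising and StopRising events.
; While rising, Tick stretches a spline mesh by lerping its end position along local X up to the given max height over the given level time.
; Overlapping it launches the PaintCharacter upward and calls PlayerDeath on the game mode.
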(event `self.ReceiveBeginPlay`
  ;[1 1 1] Initialise - create ref to self in game mode
  (bind _aspaint_mode (cast `/Game/Player/PaintMode` (`GameplayStatics.GetGameMode`)))
  (set `/Game/Player/PaintMode.FloorPaintRef` self _aspaint_mode))

(event `self.ReceiveTick`
  (params (DeltaSeconds :type "Float (single-precision)"))
  (bind _returnvalue (`SplineMeshComponent.GetStartPosition` (`self.SplineMesh1`)))
  ;[1 1 1] Rise on tick until complete
  (if (`self.Rising`)
    (bind _output_get (set `self.TimePassed` (+ DeltaSeconds (`self.TimePassed`))))
    (bind _returnvalue_2 (/ _output_get (`self.TimeToFill`)))
    (if (< _returnvalue_2 1.0)
      (`SplineMeshComponent.SetEndPosition` (`self.SplineMesh1`) (`KismetMathLibrary.VLerp` _returnvalue (`KismetMathLibrary.MakeVector` (+ (.x _returnvalue) (`self.MaxHeight`))) _returnvalue_2) true)
      (else
        (set `self.Rising` false)))))

(event `BeginRising`
  (params (MaxLevelTime :type "Float (double-precision)") (MaxPaintHeight :type "Float (double-precision)"))
  ;[1 1 1] Start Rising
  (set `self.TimeToFill` MaxLevelTime)
  (set `self.MaxHeight` MaxPaintHeight)
  (set `self.Rising` true))

(event `StopRising`
  ;[1 1 1] Stop Rising
  (set `self.Rising` false))

(event `self.SplineMesh1.OnComponentBeginOverlap`
  (params (OverlappedComponent :type "PrimitiveComponent Object Reference") (OtherActor :type "Actor Object Reference") (OtherComp :type "PrimitiveComponent Object Reference") (OtherBodyIndex :type Integer) (bFromSweep :type Boolean) (SweepResult :type "HitResult Structure (by ref)"))
  ;[1 1 1] Kill player on touch
  (bind _aspaint_character (cast `/Game/Player/PaintCharacter` OtherActor))
  (`Character.LaunchCharacter` _aspaint_character (0.0 0.0 1500.0) true true)
  (bind _aspaint_mode (cast `/Game/Player/PaintMode` (`GameplayStatics.GetGameMode`)))
  (`/Game/Player/PaintMode.PlayerDeath` _aspaint_mode))

(fn `UserConstructionScript`)