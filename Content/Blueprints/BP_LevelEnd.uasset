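; BP_LevelEnd is a level-exit trigger that ends the level when the PaintCharacter enters its box.
; On overlap it disables the character's movement, sets LevelComplete on the PaintMode game mode and shows the ContinueUI widget.
; It also turns on collision for ExpandingBox and scales that box over time with the ExpandBox timeline.
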(event `self.Box.OnComponentBeginOverlap`
  (params (OverlappedComponent :type "PrimitiveComponent Object Reference") (OtherActor :type "Actor Object Reference") (OtherComp :type "PrimitiveComponent Object Reference") (OtherBodyIndex :type Integer) (bFromSweep :type Boolean) (SweepResult :type "HitResult Structure (by ref)"))
  (bind _aspaint_character (cast `/Game/Player/PaintCharacter` OtherActor))
  (`CharacterMovementComponent.DisableMovement` (`Character.CharacterMovement` _aspaint_character))
  (bind _aspaint_mode (cast `/Game/Player/PaintMode` (`GameplayStatics.GetGameMode`)))
  (set `/Game/Player/PaintMode.LevelComplete` true _aspaint_mode)
  (bind _returnvalue (`|CreateWidget` "/Game/UI/ContinueUI.ContinueUI_C" (`GameplayStatics.GetPlayerController` 0)))
  (`UserWidget.AddToViewport` _returnvalue 0)
  (`PrimitiveComponent.SetCollisionEnabled` (`self.ExpandingBox`) "QueryAndPhysics")
  (bind (_direction _newtrack_0) (`Timeline|ExpandBox` :!via `PlayFromStart`)
    (:`Update`
      (`SceneComponent.SetWorldScale3D` (`self.ExpandingBox`) (`KismetMathLibrary.Conv_DoubleToVector` _newtrack_0)))))

(fn `UserConstructionScript`)