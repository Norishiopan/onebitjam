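; BP_WallSpline is a wall placement actor that turns a spline into a row of wall pieces.
; The construction script previews the row with M_Walls billboards, counted by spline length over BlockLength and stepped in fixed X/Z increments along the first two points' direction.
; On BeginPlay, it spawns a BP_WallPiece at each child component of Box.
; An unused spline-mesh wall branch remains disconnected.
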(event `self.ReceiveBeginPlay`
  (for _array_element (`SceneComponent.GetChildrenComponents` (`self.Box`) false)
    (`|SpawnActorFromClass` "/Game/Blueprints/BP_WallPiece.BP_WallPiece_C" (`SceneComponent.K2_GetComponentToWorld` _array_element) "Undefined" "MultiplyWithRoot" null null)))

(fn `UserConstructionScript`
  (bind _spline (`self.Spline`))
  (bind _returnvalue (`SplineComponent.GetLocationAtSplinePoint` _spline 0 "Local"))
  (for _index (range (+ (`KismetMathLibrary.FTrunc` (/ (`SplineComponent.GetSplineLength` (`self.Spline`)) (`self.BlockLength`))) 1))
    (bind _returnvalue_2 (`AddComponent|NODE_AddMaterialBillboardComponent-0` :`RelativeTransform` (`KismetMathLibrary.MakeTransform` (+ (* _index (`KismetMathLibrary.GetDirectionUnitVector` _returnvalue (`SplineComponent.GetLocationAtSplinePoint` _spline 1 "Local")) (50.0 0.0 50.0)) _returnvalue))))
    (`PrimitiveComponent.SetMaterial` _returnvalue_2 0 "/Game/Materials/M_Walls.M_Walls")))