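; Paint blob projectile that converts wall pieces, damages and knocks back enemies, and launches the player.
; Each hit plays a splat sound and casts the other actor to wall, enemy or player, destroying the bullet on a match.
; Enemies are pushed away with turning disabled, while the player is launched toward the bullet with extra lift and no damage.
; It shows a random flipbook frame, re-rolled on its single allowed bounce, and expires after a short lifetime.
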(event `self.ReceiveBeginPlay`
  ;[1 1 1] Initialise and kill after a while of no action
  (`AudioMixerBlueprintLibrary.PrimeSoundCueForPlayback` "/Game/Audio/SFX/Splat_Impact_Cue.Splat_Impact_Cue")
  (`self.RandomFrame`)
  (`KismetSystemLibrary.Delay` 5.0)
  (`self.K2_DestroyActor`))

(event `RandomFrame`
  (bind _paperflipbook (`self.PaperFlipbook`))
  ;[1 1 1] Choose a random frame for the blob to be on
  (`PaperFlipbookComponent.SetPlaybackPositionInFrames` _paperflipbook (`KismetMathLibrary.RandomIntegerInRange` 0 (- (`PaperFlipbookComponent.GetFlipbookLengthInFrames` _paperflipbook) 1)) false))

(event `self.ReceiveHit`
  (params (MyComp :type "PrimitiveComponent Object Reference") (Other :type "Actor Object Reference") (OtherComp :type "PrimitiveComponent Object Reference") (bSelfMoved :type Boolean) (HitLocation :type "Vector Structure") (HitNormal :type "Vector Structure") (NormalImpulse :type "Vector Structure") (Hit :type "HitResult Structure (by ref)"))
  (`AudioComponent.Play` (`self.Splat_Impact_Cue`) 0.0)
  ;[1 1 1] If hit a paintable surface, convert it
  (bind _asbp_wall_piece (cast `/Game/Blueprints/BP_WallPiece` Other)
    (:`then`
      (`/Game/Blueprints/BP_WallPiece.Convert` _asbp_wall_piece)
      (`self.K2_DestroyActor`))
    (:`CastFailed`
      ;[1 1 1] Knockback enemy
      (bind _asmaster_enemy (cast `/Game/Enemies/MasterEnemy` Other)
        (:`then`
          (set `/Game/Enemies/MasterEnemy.CanTurn` false _asmaster_enemy)
          (bind (_returnvalue_x _returnvalue_y _returnvalue_z) (`KismetMathLibrary.BreakVector` (* (`KismetMathLibrary.GetDirectionUnitVector` (`self.K2_GetActorLocation`) (`self.K2_GetActorLocation` _asmaster_enemy)) 250.0)))
          (`Character.LaunchCharacter` _asmaster_enemy (`KismetMathLibrary.MakeVector` _returnvalue_x 0.0 _returnvalue_z) true false)
          (`/Game/Enemies/MasterEnemy.Take Damage` _asmaster_enemy 1)
          (`self.K2_DestroyActor`))
        (:`CastFailed`
          ;[1 1 1] Knockback player
          (bind _aspaint_character (cast `/Game/Player/PaintCharacter` Other))
          (bind (_returnvalue_x_2 _returnvalue_y_2 _returnvalue_z_2) (`KismetMathLibrary.BreakVector` (* (`KismetMathLibrary.GetDirectionUnitVector` (`self.K2_GetActorLocation` _aspaint_character) (`self.K2_GetActorLocation`)) 750.0)))
          (`Character.LaunchCharacter` _aspaint_character (`KismetMathLibrary.MakeVector` _returnvalue_x_2 0.0 (+ _returnvalue_z_2 200.0)) true false)
          (`self.K2_DestroyActor`))))))

(event `self.ProjectileMovement.OnProjectileBounce`
  (params (ImpactResult :type "HitResult Structure (by ref)") (ImpactVelocity :type "Vector Structure (by ref)"))
  ;[1 1 1] Bounce (up to a limit) then destroy self
  (if (< (`self.BounceCount`) 1)
    (`self.RandomFrame`)
    (`/Engine/EditorBlueprintResources/StandardMacros.IncrementInt` (`self.BounceCount`))
    (else
      (`self.K2_DestroyActor`))))

(fn `UserConstructionScript`)